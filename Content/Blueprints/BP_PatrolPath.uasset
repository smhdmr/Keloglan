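; Patrol path Blueprint that moves a referenced Actor along its spline in an endless loop.
; The construction script snaps the Actor to the first spline point, facing along the starting tangent.
; At BeginPlay, a timeline scaled by TimelineLength starts and replays from the start whenever it finishes.
; Each update maps timeline alpha to spline distance, applies that location and rotation, then adds a fixed 90-degree local rotation offset.
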(event Custom|Play%20Timeline
  (bind _spline (Variables|Default|GetSpline))
  (bind _spline_2 (Variables|Default|GetSpline))
  ;[1 1 1] Path Follow Mehhanic
  (bind _lineartrack (Timeline|SplineTimeline PlayFromStart)
    (:Update
      (Transformation|SetActorLocationAndRotation (Variables|Default|Getactor) (Spline|GetLocationatDistanceAlongSpline _spline_2 (Math|Float|Lerp 0.0 (Spline|GetDistanceAlongSplineatSplinePoint _spline (- (Spline|GetNumberOfSplinePoints _spline) 1)) _lineartrack) "World") (Spline|GetRotationatDistanceAlongSpline _spline_2 (Math|Float|Lerp 0.0 (Spline|GetDistanceAlongSplineatSplinePoint _spline (- (Spline|GetNumberOfSplinePoints _spline) 1)) _lineartrack) "World"))
      (Transformation|AddLocalRotation (Variables|/Script/Engine.Actor|GetRootComponent (Variables|Default|Getactor)) "0.000000,-90.000000,0.000000" false false))
    (:Finished
      (CallFunction|PlayTimeline))))

(event EventBeginPlay
  ;[1 1 1] Start Path Following
  (Components|Timeline|SetPlayRate (Variables|Default|GetSplineTimeline) (/ 1.0 (Variables|Default|GettimelineLength)))
  (CallFunction|PlayTimeline))

(fn ConstructionScript
  (bind _spline (Variables|Default|GetSpline))
  ;[1 1 1] Set Begin Location and Rotation
  (Transformation|SetActorLocationAndRotation (Variables|Default|Getactor) (Spline|GetLocationatSplinePoint _spline 0 "World") (Math|Conversions|RotationFromXVector (Spline|GetTangentatDistanceAlongSpline _spline 0.0 "Local"))))