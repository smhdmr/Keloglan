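; BP_Ivy is an ivy hazard that extends when something overlaps its trigger area and damages the player through its hitbox.
; Trigger begin and end overlaps print debug messages and instantly stretch or flatten IvyParent's Z scale.
; Any overlap with IvyHitbox calls TakeDamage on player 0's HPController, without checking which actor overlapped.
; The overlap delegates are bound on Tick rather than BeginPlay.
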(event Custom|OnComponentBeginOverlap_Event
  (params (OverlappedComponent :type Primitive%20Component%20Object%20Reference) (OtherActor :type Actor%20Object%20Reference) (OtherComp :type Primitive%20Component%20Object%20Reference) (OtherBodyIndex :type Integer) (bFromSweep :type Boolean) (SweepResult :type Hit%20Result%20Structure%20%28by%20ref%29))
  ;[1 1 1] Ivy Trigger Begin Overlap
  (Development|PrintString "Entered ivy trigger")
  (Transformation|SetWorldScale3D (Variables|Default|GetIvy%20Parent) "1.000000,1.000000,5.000000"))

(event Custom|OnComponentEndOverlap_Event
  (params (OverlappedComponent :type Primitive%20Component%20Object%20Reference) (OtherActor :type Actor%20Object%20Reference) (OtherComp :type Primitive%20Component%20Object%20Reference) (OtherBodyIndex :type Integer))
  ;[1 1 1] Ivy Trigger End Overlap
  (Development|PrintString "Exited ivy trigger")
  (Transformation|SetWorldScale3D (Variables|Default|GetIvy%20Parent) "1.000000,1.000000,0.100000"))

(event Custom|CustomEvent_0
  (params (OverlappedComponent :type Primitive%20Component%20Object%20Reference) (OtherActor :type Actor%20Object%20Reference) (OtherComp :type Primitive%20Component%20Object%20Reference) (OtherBodyIndex :type Integer) (bFromSweep :type Boolean) (SweepResult :type Hit%20Result%20Structure%20%28by%20ref%29))
  ;[1 1 1] Ivy Hitbox
  (Default|TakeDamage (Actor|GetComponentbyClass (Game|GetPlayerCharacter 0) "/Game/Components/HPController.HPController_C") 1e+01))

(event EventBeginPlay)

(event Collision|EventActorBeginOverlap
  (params (OtherActor :type Actor%20Object%20Reference)))

(event EventTick
  (params (DeltaSeconds :type Float%20%28single-precision%29))
  ;[1 1 1] Ivy Trigger Begin Overlap
  (Collision|AssignOnComponentBeginOverlap (Variables|Default|GetTrigger%20Area) (delegate Custom|OnComponentBeginOverlap_Event))
  ;[1 1 1] Ivy Trigger End Overlap
  (Collision|BindEventtoOnComponentEndOverlap (Variables|Default|GetTrigger%20Area) (delegate Custom|OnComponentEndOverlap_Event))
  ;[1 1 1] Ivy Hitbox
  (Collision|AssignOnComponentBeginOverlap (Variables|Default|GetIvy%20Hitbox) (delegate Custom|CustomEvent_0)))

(fn ConstructionScript)